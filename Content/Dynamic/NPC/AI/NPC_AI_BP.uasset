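; AI controller for guard NPCs that runs the GuardBehaviour tree on the PatrolData blackboard.
; AI Perception stores sensed actors without the "Enemy" tag under EnemyKey, and clears the key on any other update.
; Every tick, the controlled Ue4ASP_Character's Aiming and Shooting flags follow whether the controller has a valid focus actor.
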(event OnTargetPerceptionUpdated(AIPerception)
  (params (Actor :type Actor%20Object%20Reference) (Stimulus :type AI%20Stimulus%20Structure))
  (bind _blackboardcomponent (Variables|Default|GetBlackboardComponent))
  (bind _enemykey (Variables|Default|GetEnemyKey))
  ;[1 1 1] On Target Perception Updated
  (if (and (not (Actor|ActorHasTag Actor "Enemy")) (.bSuccessfullySensed (Utilities|Struct|BreakAIStimulus Stimulus)))
    (AI|Components|Blackboard|SetValueasObject _blackboardcomponent _enemykey Actor)
    (else
      (AI|Components|Blackboard|ClearValue _blackboardcomponent _enemykey))))

(event EventBeginPlay
  ;[1 1 1] Begin Play
  (bind _blackboardcomponent (Class|AIController|UseBlackboard "/Game/Dynamic/NPC/AI/PatrolData.PatrolData"))
  (Variables|Default|SetBlackboardComponent _blackboardcomponent)
  (AI|RunBehaviorTree "/Game/Dynamic/NPC/AI/GuardBehaviour.GuardBehaviour"))

(event EventTick
  (params (DeltaSeconds :type Float%20%28single-precision%29))
  ;[1 1 1] Event Tick
  (bind _asue_4asp_character (Utilities|Casting|CastToUe4ASP_Character (Pawn|GetControlledPawn)))
  (bind _output_get (Variables|/Game/Dynamic/NPC/Behaviour/Ue4ASP_Character.Ue4ASP_Character_C|SetAiming _asue_4asp_character (Utilities|IsValid (Class|AIController|GetFocusActor))))
  (Variables|/Game/Dynamic/NPC/Behaviour/Ue4ASP_Character.Ue4ASP_Character_C|SetShooting _asue_4asp_character _output_get))

(fn ConstructionScript)